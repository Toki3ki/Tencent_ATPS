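; BP_Explosion_Player is a grenade explosion actor that damages zombie and human AI characters, apparently for player-thrown grenades.
; On BeginPlay it fires a RadialForce impulse and plays a 2D explosion sound.
; Overlaps on the Boom component cast to the zombie or human AI ALS character and directly subtract a fixed amount from CurrentHealth, bypassing Unreal's damage system.
; Debug prints mark the explosion and each hit.
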(event `self.ReceiveBeginPlay`
  (`KismetSystemLibrary.PrintString` "爆炸事件开始运行")
  (`RadialForceComponent.FireImpulse` (`self.RadialForce`))
  (`GameplayStatics.PlaySound2D` "/Game/Game/Sounds/Grenade/GrenadeExplosion_S08WA_229.GrenadeExplosion_S08WA_229" 1.0 1.0 0.0 null null))

(event `self.Boom.OnComponentBeginOverlap`
  (params (OverlappedComponent :type "PrimitiveComponent Object Reference") (OtherActor :type "Actor Object Reference") (OtherComp :type "PrimitiveComponent Object Reference") (OtherBodyIndex :type Integer) (bFromSweep :type Boolean) (SweepResult :type "HitResult Structure (by ref)"))
  (bind _asals_base_zombie_character_bp (cast `/Game/AdvancedLocomotionV4/Blueprints/Zombie_Logic/ALS_Base_ZOMBIE_CharacterBP` OtherActor)
    (:`then`
      (`/Engine/EditorBlueprintResources/StandardMacros.IsValid` _asals_base_zombie_character_bp
        (:`Is Valid`
          (`KismetSystemLibrary.PrintString` "爆炸伤到了丧尸")
          (set `/Game/AdvancedLocomotionV4/Blueprints/Zombie_Logic/ALS_Base_ZOMBIE_CharacterBP.Current Health` (- (`/Game/AdvancedLocomotionV4/Blueprints/Zombie_Logic/ALS_Base_ZOMBIE_CharacterBP.Current Health` _asals_base_zombie_character_bp) 1.0) _asals_base_zombie_character_bp))))
    (:`CastFailed`
      (bind _asals_human_ai_character_bp (cast `/Game/AdvancedLocomotionV4/Blueprints/Human_AI_Logic/ALS_Human_AI_CharacterBP` OtherActor))
      (`/Engine/EditorBlueprintResources/StandardMacros.IsValid` _asals_human_ai_character_bp
        (:`Is Valid`
          (`KismetSystemLibrary.PrintString` "爆炸伤到了敌军")
          (set `/Game/AdvancedLocomotionV4/Blueprints/Human_AI_Logic/ALS_BaseAI_CharacterBP.Current Health` (- (`/Game/AdvancedLocomotionV4/Blueprints/Human_AI_Logic/ALS_BaseAI_CharacterBP.Current Health` _asals_human_ai_character_bp) 1.0) _asals_human_ai_character_bp))))))

(event `self.ParticleSystem.OnParticleBurst`
  (params (EventName :type Name) (EmitterTime :type "Float (single-precision)") (ParticleCount :type Integer)))

(fn `UserConstructionScript`)